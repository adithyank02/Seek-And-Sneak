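; Sample game mode that points joining players' views at a camera it spawns itself.
; BeginPlay spawns a CameraActor at a stored transform, unhides its camera component in game and stores the actor.
; PostLogin waits briefly, then sets each valid new player's view target to that stored camera.
; Both events print debug strings.
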(event EventBeginPlay
  (bind _returnvalue (Game|SpawnActorfromClass "/Script/Engine.CameraActor" (Variables|Default|GetTans) "Undefined" "MultiplyWithRoot" 0 0))
  (Development|SetHiddeninGame (Variables|/Script/Engine.CameraActor|GetCameraComponent _returnvalue) false false)
  (if true
    (Variables|Default|SetNewVar _returnvalue)
    (Development|PrintString "Hello" true true "(R=1.000000,G=0.104572,B=0.000000,A=1.000000)")))

(event EventTick
  (params (DeltaSeconds :type Float%20%28single-precision%29)))

(event EventPostLogin
  (params (NewPlayer :type Player%20Controller%20Object%20Reference))
  (Utilities|FlowControl|Delay 0.1)
  (Utilities|IsValid NewPlayer
    (:Is%20Valid
      (Game|Player|SetViewTargetwithBlend NewPlayer (Variables|Default|GetNewVar) 0.0 "VTBlend_Linear" 0.0 false)
      (Development|PrintString "Hello"))))

(fn ConstructionScript)